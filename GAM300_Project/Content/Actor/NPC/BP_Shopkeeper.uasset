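; BP_Shopkeeper is a shopkeeper NPC that shows an input-prompt icon and relays updates to its shop UI widget.
; On BeginPlay it binds to the game mode's input-mode event, switching the icon sprite between controller and keyboard versions.
; Custom events refresh the widget's crates and raise its shop level, rebuilding items only when the new level is higher.
; UpdateShop is an empty stub.
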(event `self.ReceiveBeginPlay`
  (bind _asgam300_project_game_mode_base_bp (cast `/Game/Blueprints/GAM300_ProjectGameModeBase_BP` (`GameplayStatics.GetGameMode`)))
  (add `/Game/Blueprints/GAM300_ProjectGameModeBase_BP.UpdateInputMode` _asgam300_project_game_mode_base_bp (delegate `UpdateInputMode_Event_Shopkeeper`)))

(event `UpdateInputMode_Event_Shopkeeper`
  (params (is_controller_input :type Boolean))
  (bind _iconcomp (`self.iconComp`))
  (if is_controller_input
    (`BillboardComponent.SetSprite` _iconcomp (`self.Controller_Icon`))
    (else
      (`BillboardComponent.SetSprite` _iconcomp (`self.Keyboard_Icon`)))))

(event `self.UpdateShopCrates`
  (bind _asshop_ui (cast `/Game/UI/ShopUI_BluePrints/ShopUI` (`self.shop_widget_`)))
  (`/Game/UI/ShopUI_BluePrints/ShopUI.UpdateCrates` _asshop_ui))

(event `UpdateShop`
  (params (NewShopLevel :type Integer)))

(event `self.UpdateShopLevel`
  (params (level :type Integer))
  (bind _asshop_ui (cast `/Game/UI/ShopUI_BluePrints/ShopUI` (`self.shop_widget_`)))
  (if (> level (`/Game/UI/ShopUI_BluePrints/ShopUI.shop_level_` _asshop_ui))
    (set `/Game/UI/ShopUI_BluePrints/ShopUI.shop_level_` level _asshop_ui)
    (`/Game/UI/ShopUI_BluePrints/ShopUI.UpdateShopItems` _asshop_ui)))

(fn `UserConstructionScript`)