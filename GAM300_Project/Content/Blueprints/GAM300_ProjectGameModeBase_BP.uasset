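; Game mode that creates and manages the main UI (dialogue, tutorial, task list, portal screen) at BeginPlay, skipping the Art_Zoo level.
; It binds to ChamomileGrovePlayerController's input-device switch and relays controller versus keyboard state through CallUpdateInputMode.
; It exposes hide and unhide for the task, portal and puzzle-reset widgets, plus functions for tutorial and win-screen popups, portal reset and gamepad checks.
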(event `self.ReceiveBeginPlay`
  (`parent.ReceiveBeginPlay`)
  (bind _returnvalue (`GameplayStatics.GetCurrentLevelName` true))
  (if (not (`KismetStringLibrary.EqualEqual_StrStr` _returnvalue "Art_Zoo"))
    (`|ExecutionSequence`
      (:`then_0`
        (bind _returnvalue_2 (`|CreateWidget` "/Game/UI/DialogueUI.DialogueUI_C"))
        (bind _output_get (set `self.DialogueUI` _returnvalue_2))
        (`UserWidget.AddToViewport` _output_get 0))
      (:`then_1`
        (bind _returnvalue_3 (`|CreateWidget` "/Game/UI/TutorialScreens/Tutorial_BP.Tutorial_BP_C"))
        (bind _output_get_2 (set `self.TutorialWidget` _returnvalue_3))
        (`UserWidget.AddToViewport` _output_get_2 0))
      (:`then_2`
        (bind _returnvalue_4 (`|CreateWidget` "/Game/UI/TaskListUI.TaskListUI_C"))
        (bind _output_get_3 (set `self.TaskWidget` _returnvalue_4)))
      (:`then_3`
        (bind _returnvalue_5 (`|CreateWidget` "/Game/UI/PocketPortalUI/PortalScreenUI.PortalScreenUI_C"))
        (bind _output_get_4 (set `self.PortalWidget` _returnvalue_5))
        (`KismetSystemLibrary.Delay` 5.0)
        (`UserWidget.AddToViewport` _output_get_4 0))
      (:`then_4`
        (`self.UnhideUI`))
      (:`then_5`
        (bind _aschamomile_grove_player_controller (cast `/Game/Blueprints/ChamomileGrovePlayerController` (`GameplayStatics.GetPlayerController` 0)))
        (add `/Game/Blueprints/ChamomileGrovePlayerController.SwitchedInputDevice` _aschamomile_grove_player_controller (delegate `SwitchedInputDevice_Event_GameMode`))))))

(event `SwitchedInputDevice_Event_GameMode`
  (params (is_controller :type Boolean))
  (bind _output_get (set `self.is_controller_used` is_controller))
  (`self.UpdateInputMode` _output_get))

(event `self.ReceiveTick`
  (params (DeltaSeconds :type "Float (single-precision)")))

(event `InputModeCall`
  (`self.UpdateInputMode` (`self.is_controller_used`)))

(event `self.HideUI`
  (`|ExecutionSequence`
    (:`then_0`
      (`Widget.SetVisibility` (`self.TaskWidget`) "Hidden"))
    (:`then_3`
      (`Widget.SetVisibility` (`self.PortalWidget`) "Hidden"))
    (:`then_4`
      (bind _foundwidgets (`WidgetBlueprintLibrary.GetAllWidgetsOfClass` "/Game/UI/ResetPuzzle.ResetPuzzle_C"))
      (bind _asreset_puzzle (cast `/Game/UI/ResetPuzzle` (`|GetArrayItem` _foundwidgets)))
      (`Widget.SetVisibility` _asreset_puzzle "Hidden"))))

(event `self.UnhideUI`
  (`|ExecutionSequence`
    (:`then_0`
      (`Widget.SetVisibility` (`self.TaskWidget`) "SelfHitTestInvisible"))
    (:`then_3`
      (`Widget.SetVisibility` (`self.PortalWidget`) "SelfHitTestInvisible"))
    (:`then_4`
      (bind _foundwidgets (`WidgetBlueprintLibrary.GetAllWidgetsOfClass` "/Game/UI/ResetPuzzle.ResetPuzzle_C"))
      (bind _asreset_puzzle (cast `/Game/UI/ResetPuzzle` (`|GetArrayItem` _foundwidgets)))
      (`Widget.SetVisibility` _asreset_puzzle "SelfHitTestInvisible"))))

(fn `CheckController`
  (bind _returnvalue (`self.IsGamePadConnected`))
  (if (!= _returnvalue (`self.is_controller_used`))
    (bind _output_get (set `self.is_controller_used` _returnvalue))
    (`self.UpdateInputMode` _output_get)))

(fn `PopUpCraftingTutorial`
  (bind _tutorialwidget (`self.TutorialWidget`))
  (set `/Game/UI/TutorialScreens/Tutorial_BP.curPT` 0 _tutorialwidget)
  (for _array_element (`/Game/UI/TutorialScreens/Tutorial_BP.CraftingSlides_Controller` _tutorialwidget)
    (`Widget.SetVisibility` _array_element "Hidden"))
  (for _array_element_2 (`/Game/UI/TutorialScreens/Tutorial_BP.CraftingSlides_Key` _tutorialwidget)
    (`Widget.SetVisibility` _array_element_2 "Hidden"))
  (`/Game/UI/TutorialScreens/Tutorial_BP.Event Start Potion Tutorial` _tutorialwidget))

(fn `PopUpFarmingTutorial`
  (bind _tutorialwidget (`self.TutorialWidget`))
  (set `/Game/UI/TutorialScreens/Tutorial_BP.curFT` 0 _tutorialwidget)
  (for _array_element (`/Game/UI/TutorialScreens/Tutorial_BP.FarmingSlides_Key` _tutorialwidget)
    (`Widget.SetVisibility` _array_element "Hidden"))
  (for _array_element_2 (`/Game/UI/TutorialScreens/Tutorial_BP.FarmingSlides_Controller` _tutorialwidget)
    (`Widget.SetVisibility` _array_element_2 "Hidden"))
  (`/Game/UI/TutorialScreens/Tutorial_BP.Event Start Farming Tutorial` _tutorialwidget)
  (`/Game/UI/TutorialScreens/Tutorial_BP.EventReset` _tutorialwidget))

(fn `PopUpWinScreen`
  (`/Game/UI/TutorialScreens/Tutorial_BP.Event Start Win Screen` (`self.TutorialWidget`)))

(fn `ResetPocketPortal`
  (`/Game/UI/PocketPortalUI/PortalScreenUI.EventReset` (`self.PortalWidget`)))

(fn `UserConstructionScript`
  (`parent.UserConstructionScript`))