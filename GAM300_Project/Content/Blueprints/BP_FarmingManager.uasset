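; Farming manager actor that watches every BP_FarmingPlot3 in the level to drive plants-ready audio and track first-time farming milestones.
; BeginPlay gathers the plots, starts a looping-state Wwise event and resets the milestone flags.
; Tick recounts harvestable plots, sending changes to the PlantsReady RTPC with interpolation.
; Tick also scans plots for first water, harvest and plant, latching each manager flag through a DoOnce.
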(event `self.ReceiveBeginPlay`
  ;[1 1 1] Get all farming plots in game
  (`|ExecutionSequence`
    (:`then_0`
      (bind _outactors (`GameplayStatics.GetAllActorsOfClass` "/Game/Blueprints/BP_FarmingPlot3.BP_FarmingPlot3_C"))
      (set `self.Plots` _outactors)
      ;[1 1 1] Start playing the Item Ready sound and set it to be silent at the start
      (`AkGameplayStatics.PostEventAtLocation` "/Game/WwiseAudio/Events/Default_Work_Unit/StartItemPlantsReady.StartItemPlantsReady" (-330.0 -20.0 10.0) (`PlayerCameraManager.GetCameraRotation` (`GameplayStatics.GetPlayerCameraManager` 0)))
      (`AkGameplayStatics.SetRTPCValue` "/Game/WwiseAudio/Game_Parameters/Default_Work_Unit/PlantsReady.PlantsReady")
      (set `self.FirstWatered` false)
      (set `self.FirstHarvest` false)
      (set `self.FirstPlant` false))
    (:`then_1`
      (goto _label :!via `Reset`))
    (:`then_2`
      (goto _label_2 :!via `Reset`))
    (:`then_3`
      (goto _label_3 :!via `Reset`))))

(event `self.ReceiveTick`
  (params (DeltaSeconds :type "Float (single-precision)"))
  (`|ExecutionSequence`
    (:`then_0`
      ;[1 1 1] Count the number of harvestable plants
      (set `self.PrevCount` (`self.CurCount`) :!pinned true) ; Store the count from the last frame
      (set `self.CurCount` 0)
      (for _array_element (`self.Plots`)
        (if (`FarmingPlot.b_harvestable_` _array_element)
          (bind _result (`/Engine/EditorBlueprintResources/StandardMacros.IncrementInt` (`self.CurCount`))
            (:`  `
              (set `self.CurCount` _result)))))
      ;[1 1 1] Check if number of harvestable plants changed
      (if (!= (`self.PrevCount`) (`self.CurCount`))
        ;[1 1 1] Update RTPC value
        (`AkGameplayStatics.SetRTPCValue` "/Game/WwiseAudio/Game_Parameters/Default_Work_Unit/PlantsReady.PlantsReady" (`KismetMathLibrary.Conv_IntToDouble` (`self.CurCount`)) 1000)))
    (:`then_1`
      (if (not (`self.FirstWatered`))
        ;[1 1 1] Player first watered
        (for _array_element_2 (`self.Plots`)
          (bind _b_first_water_ (`FarmingPlot.b_first_water_` _array_element_2))
          (if _b_first_water_
            (break)))
        (if _b_first_water_
          (`/Engine/EditorBlueprintResources/StandardMacros.DoOnce` false :!label _label
            (:`Completed`
              (set `self.FirstWatered` true))))))
    (:`then_2`
      (if (not (`self.FirstHarvest`))
        ;[1 1 1] Player first harvest
        (for _array_element_3 (`self.Plots`)
          (bind _b_first_harvest_ (`FarmingPlot.b_first_harvest_` _array_element_3))
          (if _b_first_harvest_
            (break)))
        (if _b_first_harvest_
          (`/Engine/EditorBlueprintResources/StandardMacros.DoOnce` false :!label _label_2
            (:`Completed`
              (set `self.FirstHarvest` true))))))
    (:`then_3`
      (if (not (`self.FirstPlant`))
        ;[1 1 1] Player first harvest
        (for _array_element_4 (`self.Plots`)
          (bind _b_first_plant_ (`FarmingPlot.b_first_plant_` _array_element_4))
          (if _b_first_plant_
            (break)))
        (if _b_first_plant_
          (`/Engine/EditorBlueprintResources/StandardMacros.DoOnce` false :!label _label_3
            (:`Completed`
              (set `self.FirstPlant` true))))))))

(fn `UserConstructionScript`)