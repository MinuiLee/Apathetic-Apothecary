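; BP_River is a river actor that plays a Wwise water splash sound when a CharacterBase begins overlapping it.
; The PlayerWaterSplash event is posted at the world origin rather than at the overlapping character.
; A cooldown timer, set after a short delay and counted down on Tick, blocks repeat splashes until it reaches zero.
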(event `self.ReceiveActorBeginOverlap`
  (params (OtherActor :type "Actor Object Reference"))
  (if (== (`self.timer`) 0.0)
    (cast `CharacterBase` OtherActor)
    (`AkGameplayStatics.PostEventAtLocation` "/Game/WwiseAudio/Events/Default_Work_Unit/PlayerWaterSplash.PlayerWaterSplash")
    (`KismetSystemLibrary.Delay` 0.2)
    (set `self.timer` 0.5)))

(event `self.ReceiveTick`
  (params (DeltaSeconds :type "Float (single-precision)"))
  (set `self.timer` (`KismetMathLibrary.FMax` (- (`self.timer`) DeltaSeconds))))

(fn `UserConstructionScript`)