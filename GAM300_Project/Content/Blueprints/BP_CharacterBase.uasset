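; Base player character for a farming and potion game, bridging gameplay actions to Camille's animation Blueprint.
; Action events set animation flags, most gated on InBlockingState, with planting, watering, potion and lift actions also stopping movement.
; BeginPlay creates scene-fade, puzzle-reset and cheat widgets; door fades toggle input.
; It also detects gamepad/keyboard switches and provides freeze, hand-attach and conversation helpers, while camera zoom and rotate-to-face logic are disconnected.
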(event `Dialogue_Interface.OnInteract`
  (params (Caller :type "Character Object Reference"))
  (message `ItemInterface.OnInteract` Caller null))

(event `self.ReceiveBeginPlay`
  ;[1 1 1] Begin play, also adds a reference to the animation
  (`parent.ReceiveBeginPlay`)
  (bind _asabp_camille_final (cast `/Game/Animations/AnimationBlueprint/ABP_Camille_Final` (`SkeletalMeshComponent.GetAnimInstance` (`self.Mesh`))))
  (bind _output_get (set `self.AnimationBP` _asabp_camille_final))
  (set `/Game/Animations/AnimationBlueprint/ABP_Camille_Final.Character` self _output_get)
  (`AkGameplayStatics.SetState` "/Game/WwiseAudio/States/Default_Work_Unit/Music/Music-Farm.Music-Farm")
  (bind _returnvalue (`|CreateWidget` "/Game/UI/Loading_Blueprints/SceneTransition.SceneTransition_C" (`GameplayStatics.GetPlayerController` 0)))
  (bind _output_get_2 (set `self.Fade` _returnvalue))
  (`self.DoorFadeBind`)
  (`UserWidget.AddToViewport` _output_get_2 100)
  (bind _returnvalue_2 (`|CreateWidget` "/Game/UI/ResetPuzzle.ResetPuzzle_C"))
  (bind _output_get_3 (set `self.ResetPuzzleMenu` _returnvalue_2))
  (`UserWidget.AddToViewport` _output_get_3 0)
  (bind _returnvalue_3 (`|CreateWidget` "/Game/UI/CheatMenu.CheatMenu_C"))
  (bind _output_get_4 (set `self.CheatMenu` _returnvalue_3))
  (`KismetSystemLibrary.Delay` 0.1)
  (`UserWidget.AddToViewport` _output_get_4 0))

(event `self.PlantEvent`
  (params (plot :type "Actor Object Reference"))
  (bind _animationbp (`self.AnimationBP`))
  ;[1 1 1] Plant animaion call
  (if (not (`/Game/Animations/AnimationBlueprint/ABP_Camille_Final.in_Blocking_State` _animationbp))
    (set `/Game/Animations/AnimationBlueprint/ABP_Camille_Final.is_planting` true _animationbp)
    (set `self.animationFocus` plot)
    (`InventoryComponent.SetLock` (`self.inventoryComp`) true)
    (`self.DisableMovementInput` true)
    (set `MovementComponent.Velocity` (0.0 0.0 0.0) (`self.GetMovementComponent`))))

(event `RepositionEnd`
  ;[1 1 1] Plant animaion call
)

(event `Reposition`
  (params (Output :type "Float (double-precision)"))
  ;[1 1 1] Plant animaion call
  (`/Game/Blueprints/FunctionLibraries/BP_HelperFunctions.Trans Rot To Actor` self (`self.K2_GetActorLocation` (stale `self.PlantEvent` plot)) 2.0 25.0))

(event `self.EventUsePotionSelf`
  ;[1 1 1] Potion drink setup
  (if (not (`/Game/Animations/AnimationBlueprint/ABP_Camille_Final.in_Blocking_State` (`self.AnimationBP`)))
    (set `/Game/Animations/AnimationBlueprint/ABP_Camille_Final.is_drinking_potion` true (`self.AnimationBP`))
    (`InventoryComponent.SetLock` (`self.inventoryComp`) true)
    (`self.DisableMovementInput` true)
    (set `MovementComponent.Velocity` (0.0 0.0 0.0) (`self.GetMovementComponent`))))

(event `self.AnimWaterPlot`
  (params (plot :type "Actor Object Reference"))
  ;[1 1 1] Water plot animation setup
  (if (not (`/Game/Animations/AnimationBlueprint/ABP_Camille_Final.in_Blocking_State` (`self.AnimationBP`)))
    (set `/Game/Animations/AnimationBlueprint/ABP_Camille_Final.is_watering` true (`self.AnimationBP`))
    (set `self.animationFocus` plot)
    (`InventoryComponent.SetLock` (`self.inventoryComp`) true)
    (`self.DisableMovementInput` true)
    (set `MovementComponent.Velocity` (0.0 0.0 0.0) (`self.GetMovementComponent`))))

(event `WaterPlotTransitionEnd`
  ;[1 1 1] Water plot animation setup
)

(event `WaterPlotTransition`
  (params (Output :type "Float (double-precision)"))
  ;[1 1 1] Water plot animation setup
  (`/Game/Blueprints/FunctionLibraries/BP_HelperFunctions.Trans Rot To Actor` self (`self.K2_GetActorLocation` (stale `self.AnimWaterPlot` plot)) 2.0 25.0))

(event `self.AnimUsePotionObject`
  (params (actor :type "Actor Object Reference"))
  ;[1 1 1] Use potion on object animation setup
  (if (not (`/Game/Animations/AnimationBlueprint/ABP_Camille_Final.in_Blocking_State` (`self.AnimationBP`)))
    (set `/Game/Animations/AnimationBlueprint/ABP_Camille_Final.is_pouring_potion` true (`self.AnimationBP`))
    (set `self.animationFocus` actor)
    (`InventoryComponent.SetLock` (`self.inventoryComp`) true)
    (`self.DisableMovementInput` true)
    (set `MovementComponent.Velocity` (0.0 0.0 0.0) (`self.GetMovementComponent`))))

(event `PotionObjectTransitionEnd`
  ;[1 1 1] Use potion on object animation setup
)

(event `PotionObjectTransition`
  (params (Output :type "Float (double-precision)"))
  ;[1 1 1] Use potion on object animation setup
  (`/Game/Blueprints/FunctionLibraries/BP_HelperFunctions.Trans Rot To Actor` self (`self.K2_GetActorLocation` (stale `self.AnimUsePotionObject` actor)) 2.0 25.0))

(event `self.AnimLift`
  (params (Item :type "Actor Object Reference"))
  (if (not (`/Game/Animations/AnimationBlueprint/ABP_Camille_Final.in_Blocking_State` (`self.AnimationBP`)))
    (set `/Game/Animations/AnimationBlueprint/ABP_Camille_Final.is_lifting` true (`self.AnimationBP`))
    (set `self.animationFocus` Item)
    (`self.DisableMovementInput` true)
    (set `MovementComponent.Velocity` (0.0 0.0 0.0) (`self.GetMovementComponent`))))

(event `self.AnimThrow`
  (if (not (`/Game/Animations/AnimationBlueprint/ABP_Camille_Final.in_Blocking_State` (`self.AnimationBP`)))
    (set `/Game/Animations/AnimationBlueprint/ABP_Camille_Final.is_throwing` true (`self.AnimationBP`))))

(event `self.AnimDrop`
  (if (not (`/Game/Animations/AnimationBlueprint/ABP_Camille_Final.in_Blocking_State` (`self.AnimationBP`)))
    (set `/Game/Animations/AnimationBlueprint/ABP_Camille_Final.is_dropping` true (`self.AnimationBP`))))

(event `self.FreezeFloatingPlatform`
  (params (platform :type "Actor Object Reference"))
  (bind _asmoving_platform (cast `/Game/Blueprints/PuzzleObjects/MovingPlatform` platform))
  (set `/Game/Blueprints/PuzzleObjects/MovingPlatform.TimeStopTimeLeft` 5.0 _asmoving_platform))

(event `self.DoorFade`
  (bind _fade (`self.Fade`))
  ;[1 1 1] Door fade section
  (`/Game/UI/Loading_Blueprints/SceneTransition.BindFunctions` _fade)
  (`/Game/UI/Loading_Blueprints/SceneTransition.OnFade` _fade)
  (`self.DisableInput` (`GameplayStatics.GetPlayerController` 0))
  (set `MovementComponent.Velocity` (0.0 0.0 0.0) (`self.GetMovementComponent`)))

(event `DoorFadeBind`
  (bind _fade (`self.Fade`))
  ;[1 1 1] Door fade section
  (add `/Game/UI/Loading_Blueprints/SceneTransition.FadeInFinished` _fade (delegate `FadeInFinished_Event_0`))
  (add `/Game/UI/Loading_Blueprints/SceneTransition.FadeOutFinished` _fade (delegate `FadeOutFinished_Event_0`)))

(event `FadeInFinished_Event_0`
  ;[1 1 1] Door fade section
  (`self.DoorFadeInFinished`))

(event `FadeOutFinished_Event_0`
  ;[1 1 1] Door fade section
  (`self.DoorFadeOutFinished`)
  (`Widget.SetVisibility` (`self.Fade`) "Hidden")
  (`self.EnableInput` (`GameplayStatics.GetPlayerController` 0)))

(event `OnLevelClose`
  (`InventoryComponent.RemoveInventoryHUD` (`self.inventoryComp`)))

(event `self.ReceiveEndPlay`
  (params (EndPlayReason :type "EEndPlayReason Enum" :default "Destroyed"))
  (`Widget.RemoveFromParent` (`self.CheatMenu`))
  (`Widget.RemoveFromParent` (`self.ResetPuzzleMenu`)))

(event `Key|AnyKey`
  (params (Key :type "Key Structure"))
  (bind _returnvalue (`KismetInputLibrary.Key_IsGamepadKey` Key))
  ;[1 1 1] Detect if using Keyboard or Gamepad
  (:`Pressed`
    (if (!= _returnvalue (`self.b_gamepad`))
      (set `self.b_gamepad` _returnvalue)
      (`TicketComponent.ResetRecipeBook` (`self.ticketComp`))
      (`self.ResetCrate`))))

(event `InputAxis|CameraZoom`
  (params (AxisValue :type "Float (single-precision)"))
  ;[1 1 1] Camera Zoom
)

(event `self.AnimPush`
  (params (pushing :type Boolean))
  (set `/Game/Animations/AnimationBlueprint/ABP_Camille_Final.is_pushing` pushing (`self.AnimationBP`)))

(fn `AttachComponent`
  (params (Actor :type "Actor Object Reference"))
  (`SceneComponent.K2_AttachToComponent` (`Actor.RootComponent` Actor) (`self.Mesh`) "R_palm_jnt" "SnapToTarget" "KeepRelative" "KeepWorld" true))

(fn `DetachComponent`
  (params (Actor :type "Actor Object Reference"))
  (`self.K2_DetachFromActor` Actor "KeepWorld" "KeepRelative" "KeepWorld"))

(fn `FreezePlayer`
  (`InventoryComponent.SetLock` (`self.inventoryComp`) true)
  (`self.DisableMovementInput` true)
  (set `MovementComponent.Velocity` (0.0 0.0 0.0) (`self.GetMovementComponent`))
  (set `self.b_canInteract` false))

(fn `GetSkeletalMesh`
  (returns (SkeletalMesh :type "SkeletalMeshComponent Object Reference"))
  (return (`self.Mesh`)))

(fn `SetInConversation`
  (params (in_conversation :type Boolean))
  (set `/Game/Animations/AnimationBlueprint/ABP_Camille_Final.is_in_conversation` in_conversation (`self.AnimationBP`)))

(fn `TalkAnimation`
  (set `/Game/Animations/AnimationBlueprint/ABP_Camille_Final.is_talking` true (`self.AnimationBP`)))

(fn `UnFreezePlayer`
  (`InventoryComponent.SetLock` (`self.inventoryComp`) false)
  (`self.DisableMovementInput` false)
  (set `MovementComponent.Velocity` (0.0 0.0 0.0) (`self.GetMovementComponent`))
  (set `self.b_canInteract` true))

(fn `UserConstructionScript`
  (`parent.UserConstructionScript`))