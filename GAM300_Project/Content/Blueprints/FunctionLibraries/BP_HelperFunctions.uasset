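; Blueprint function library with helpers for positioning characters and driving acknowledge animations, including for dialogue.
; TransRotToActor moves a character at constant interpolation speed toward a set horizontal distance from a target location while turning its yaw to face it.
; DialogueAnimationAcknowledge tries casts to the Aoife, Ellias, Fiz and Shopkeeper Anim Blueprints to set their acknowledge flag.
; CharacterAnimationAcknowledge only casts to Camille's Anim Blueprint and sets nothing on it.
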(fn `CharacterAnimationAcknowledge`
  (params (Mesh :type "SkeletalMeshComponent Object Reference") (ack :type Boolean))
  (locals (Character_ack :type Boolean))
  (set `local.Character_ack` ack)
  (cast `/Game/Animations/AnimationBlueprint/ABP_Camille_Final` (`SkeletalMeshComponent.GetAnimInstance` Mesh)))

(fn `DialogueAnimationAcknowledge`
  (params (NPC_Mesh :type "SkeletalMeshComponent Object Reference (by ref)") (acknowledge :type Boolean))
  (locals (Ack :type Boolean))
  (bind _returnvalue (`SkeletalMeshComponent.GetAnimInstance` NPC_Mesh))
  (set `local.Ack` acknowledge)
  (bind _asabp_aoife (cast `/Game/Animations/AnimationBlueprint/ABP_Aoife` _returnvalue)
    (:`then`
      (set `/Game/Animations/AnimationBlueprint/ABP_Aoife.acknowledge` (`local.Ack`) _asabp_aoife))
    (:`CastFailed`
      (bind _asabp_ellias (cast `/Game/Animations/AnimationBlueprint/ABP_Ellias` _returnvalue)
        (:`then`
          (set `/Game/Animations/AnimationBlueprint/ABP_Ellias.acknoledge` (`local.Ack`) _asabp_ellias))
        (:`CastFailed`
          (bind _asabp_fiz (cast `/Game/Animations/AnimationBlueprint/ABP_Fiz` _returnvalue)
            (:`then`
              (set `/Game/Animations/AnimationBlueprint/ABP_Fiz.acknowledge` (`local.Ack`) _asabp_fiz))
            (:`CastFailed`
              (bind _asabp_shopkeeper (cast `/Game/Animations/AnimationBlueprint/ABP_Shopkeeper` _returnvalue))
              (set `/Game/Animations/AnimationBlueprint/ABP_Shopkeeper.acknowledge` (`local.Ack`) _asabp_shopkeeper))))))))

(fn `Trans Rot To Actor`
  (params (Character :type "/Game/Blueprints/BP_CharacterBase Object Reference") (ActorLocation :type "Vector Structure") (InterSpeed :type "Float (double-precision)") (Distance :type "Float (double-precision)"))
  (locals (Rotator :type "Rotator Structure") (CharLocation :type "Vector Structure"))
  (bind (_returnvalue_roll _returnvalue_pitch _returnvalue_yaw) (`KismetMathLibrary.BreakRotator` (`KismetMathLibrary.FindLookAtRotation` (`local.CharLocation`) ActorLocation)))
  (bind _returnvalue (`KismetMathLibrary.MakeRotator` 0.0 0.0 _returnvalue_yaw))
  (bind _output_get (set `local.CharLocation` (`Actor.K2_GetActorLocation` Character)))
  (bind _returnvalue_2 (`KismetMathLibrary.Normal` (- _output_get ActorLocation)))
  (if (== _returnvalue_2 (0.0 0.0 0.0))
    (set `local.Rotator` _returnvalue)
    (else
      (set `local.Rotator` (`KismetMathLibrary.RInterpTo_Constant` (`Actor.K2_GetActorRotation` Character) _returnvalue (`GameplayStatics.GetWorldDeltaSeconds` null) InterSpeed))))
  (bind (_returnvalue_x _returnvalue_y) (`KismetMathLibrary.BreakVector` (+ (* _returnvalue_2 Distance) ActorLocation)))
  (`Actor.K2_SetActorLocationAndRotation` Character (`KismetMathLibrary.VInterpTo_Constant` (`local.CharLocation`) (`KismetMathLibrary.MakeVector` _returnvalue_x _returnvalue_y (.z (`local.CharLocation`))) (`GameplayStatics.GetWorldDeltaSeconds` null) InterSpeed) (`local.Rotator`) false false))