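; ChamomileGrovePlayerController is a player controller that tracks whether the player is using a gamepad or keyboard and mouse.
; An AnyKey press checks if the key belongs to the keyboard or mouse, treating any other key as controller input.
; When the device type changes, it flips the IsController flag and calls the SwitchedInputDevice dispatcher with the new value, so repeated input from the same device triggers nothing.
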(event `Key|AnyKey` :consume false :paused true
  (params (Key :type "Key Structure"))
  (:`Pressed`
    (if (or (`KismetInputLibrary.Key_IsKeyboardKey` Key) (`KismetInputLibrary.Key_IsMouseButton` Key))
      (if (`self.is_controller`)
        (bind _output_get (set `self.is_controller` false))
        (`self.SwitchedInputDevice` _output_get))
      (elif (not (`self.is_controller`))
        (bind _output_get_2 (set `self.is_controller` true))
        (`self.SwitchedInputDevice` _output_get_2)))))

(fn `UserConstructionScript`)