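; BP_FarmingPlot3 is a farming plot actor that keeps its crop UI prompt matched to the active input device.
; On BeginPlay it caches GameStats and registers an event with the game mode, which forwards controller or non-controller changes to the CropUI widget's sprite swap.
; Tick checks watered and harvested flags, but both branches are empty and the PS_Growth particle spawns meant for them are disconnected.
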(event `self.ReceiveBeginPlay`
  (bind _returnvalue (`GameplayStatics.GetActorOfClass` "/Script/GAM300_Project.GameStats"))
  (set `self.game_stats_` _returnvalue)
  (bind _asgam300_project_game_mode_base_bp (cast `/Game/Blueprints/GAM300_ProjectGameModeBase_BP` (`GameplayStatics.GetGameMode`)))
  (add `/Game/Blueprints/GAM300_ProjectGameModeBase_BP.UpdateInputMode` _asgam300_project_game_mode_base_bp (delegate `UpdateInputMode_Event_Platform`)))

(event `UpdateInputMode_Event_Platform`
  (params (is_controller_input :type Boolean))
  (`self.ChangeInputSprite` is_controller_input))

(event `self.ReceiveTick`
  (params (DeltaSeconds :type "Float (single-precision)"))
  (`|ExecutionSequence`
    (:`then_0`
      ;[1 1 1] Water Plot Particles
      ;;[1 1 1] If Plot watered
      (if (`self.b_watered_this_frame_`)
        _))
    (:`then_1`
      ;[1 1 1] Harvest plant particles
      ;;[1 1 1] If plant harvested on plot
      (if (`self.b_harvested_this_frame_`)
        _))))

(fn `ChangeInputSprite`
  (params (is_controller :type Boolean))
  (bind _ascrop_ui (cast `/Game/UI/FarmingUI_BluePrints/CropUI` (`WidgetComponent.GetUserWidgetObject` (`self.widgetComp`))))
  (`/Game/UI/FarmingUI_BluePrints/CropUI.Change Input Sprite` _ascrop_ui is_controller))

(fn `UserConstructionScript`)