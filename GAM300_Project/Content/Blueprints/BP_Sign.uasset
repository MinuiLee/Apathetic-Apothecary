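; BP_Sign is a sign Blueprint that shows or hides a dialogue widget on screen when its InteractDia event fires.
; The event removes and clears an existing widget, or creates one for the first player controller and adds it to the viewport.
; The widget receives a hardcoded "Press E to Talk" message, while the assignment of SignText to its DialogueText is disconnected and never runs.
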(event `/Game/Dialogue/Interact_Dia.Interact_Dia`
  (`/Engine/EditorBlueprintResources/StandardMacros.IsValid` (`self.Dialogue_Widget`)
    (:`Is Valid`
      (`Widget.RemoveFromParent` (`self.Dialogue_Widget`))
      (set `self.Dialogue_Widget` null))
    (:`Is Not Valid`
      (bind _returnvalue (`|CreateWidget` "/Game/Dialogue/DialogueWidget.DialogueWidget_C" (`GameplayStatics.GetPlayerController` 0) "Press E to Talk"))
      (bind _output_get (set `self.Dialogue_Widget` _returnvalue))
      (`UserWidget.AddToViewport` _output_get 0))))

(fn `UserConstructionScript`)