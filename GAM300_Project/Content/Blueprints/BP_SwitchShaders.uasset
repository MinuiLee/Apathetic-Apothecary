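; Blueprint actor that toggles a post-process shader effect on and off when an actor overlaps it, with a text label.
; On BeginPlay it casts its widget component's user widget to Text and sets the displayed string from TextToDisplay.
; Each overlap runs a FlipFlop that switches the PostProcess blend weight between zero and full, starting with off.
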(event `self.ReceiveBeginPlay`
  (bind _astext (cast `/Game/UI/Widget_Helpers/Text` (`WidgetComponent.GetUserWidgetObject` (`self.Widget`))))
  (bind _output_get (set `self.Text` _astext))
  (`TextBlock.SetText` (`/Game/UI/Widget_Helpers/Text.TextBlock_124` _output_get) (`self.Text_To_Display`)))

(event `self.ReceiveActorBeginOverlap`
  (params (OtherActor :type "Actor Object Reference"))
  (bind _postprocess (`self.PostProcess`))
  (`/Engine/EditorBlueprintResources/StandardMacros.FlipFlop`
    (:`A`
      (set `PostProcessComponent.BlendWeight` 0.0 _postprocess))
    (:`B`
      (set `PostProcessComponent.BlendWeight` 1.0 _postprocess))))

(fn `UserConstructionScript`)