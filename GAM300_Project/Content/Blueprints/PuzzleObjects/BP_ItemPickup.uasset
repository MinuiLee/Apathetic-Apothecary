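; BP_ItemPickup is a puzzle item pickup that can end the game when it belongs to the last puzzle.
; On BeginPlay it runs the parent logic and registers with the game mode for input-mode updates, switching its prompt sprite between controller and other input.
; Its GameEnd event, if IsLastPuzzle is set, flags the game as won on the ChamomileGrove game instance and loads the credits level through it.
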(event `self.ReceiveBeginPlay`
  (`parent.ReceiveBeginPlay`)
  (bind _asgam300_project_game_mode_base_bp (cast `/Game/Blueprints/GAM300_ProjectGameModeBase_BP` (`GameplayStatics.GetGameMode`)))
  (add `/Game/Blueprints/GAM300_ProjectGameModeBase_BP.UpdateInputMode` _asgam300_project_game_mode_base_bp (delegate `UpdateInputMode_Event_Platform`)))

(event `UpdateInputMode_Event_Platform`
  (params (is_controller_input :type Boolean))
  (`self.ChangeInputSprite` is_controller_input))

(event `self.GameEnd`
  (if (`self.isLastPuzzle`)
    (bind _aschamomile_grove_instance_bp (cast `/Game/Blueprints/ChamomileGroveInstance_BP` (`GameplayStatics.GetGameInstance`)))
    (set `/Game/Blueprints/ChamomileGroveInstance_BP.won_game_` true _aschamomile_grove_instance_bp)
    (`/Game/Blueprints/ChamomileGroveInstance_BP.LoadStreamLevel` _aschamomile_grove_instance_bp "CreditsScreen")))

(fn `UserConstructionScript`)