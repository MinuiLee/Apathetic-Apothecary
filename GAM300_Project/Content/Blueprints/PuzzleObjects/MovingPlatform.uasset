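; A puzzle platform that shuttles back and forth between its start and a Destination point, with support for being paused by time stop.
; Tick moves it at constant speed, waits a cooldown at each end, and halts while TimeStopTimeLeft, set outside this graph, counts down.
; When it is the player's current hit actor, a prompt shows the held potion's rescaled icon, crossed out unless the potion has one specific effect.
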(event `self.ReceiveBeginPlay`
  ;[1 1 1] Set up variables
  (set `self.PointA` (`SceneComponent.K2_GetComponentLocation` (`self.Platform`)))
  (bind _output_get (set `self.PointB` (`SceneComponent.K2_GetComponentLocation` (`self.Destination`))))
  (set `self.Target` _output_get)
  (set `self.Cooldown` (`self.CooldownLength`))
  (set `self.DefaultIcon` (`BillboardComponent.Sprite` (`self.Icon`))))

(event `self.ReceiveTick`
  (params (DeltaSeconds :type "Float (single-precision)"))
  (bind _platform (`self.Platform`))
  (bind _cooldown (`self.Cooldown`))
  (bind _timestoptimeleft (`self.TimeStopTimeLeft`))
  (bind _x (`self.X`))
  (bind _icon (`self.Icon`))
  (bind _newsprite (`self.NewSprite`))
  (bind _returnvalue (`SceneComponent.K2_GetComponentLocation` _platform))
  (bind _returnvalue_2 (/ (* (.x (`SceneComponent.K2_GetComponentScale` _icon)) (`KismetMathLibrary.Conv_IntToDouble` (`Texture2D.Blueprint_GetSizeX` (`BillboardComponent.Sprite` _icon)))) (`KismetMathLibrary.Conv_IntToDouble` (`Texture2D.Blueprint_GetSizeX` _newsprite))))
  ;[1 1 1] Move platform
  (bind _ascharacter_base (cast `CharacterBase` (`GameplayStatics.GetPlayerCharacter` 0)))
  (bind _returnvalue_3 (`CharacterBase.GetCurrentHitActor` _ascharacter_base))
  (bind _returnvalue_4 (== _returnvalue_3 self))
  (`SceneComponent.SetVisibility` (`self.prompt`) _returnvalue_4 true)
  (if _returnvalue_4
    (bind _asda_potion (cast `DA_Potion` (`.itemType_` (break `US_Item` (`InventoryComponent.GetCurrentItem` (`CharacterBase.inventoryComp` _ascharacter_base)))))
      (:`then`
        (`SceneComponent.SetVisibility` _x (not (== (`DA_Potion.potion_effect_` _asda_potion) (cast `E_POTION_EFFECT` 4))) false)
        (set `self.NewSprite` (`DA_Potion.texture_` _asda_potion)))
      (:`CastFailed`
        (`SceneComponent.SetVisibility` _x true false)
        (set `self.NewSprite` (`self.DefaultIcon`))))
    (`SceneComponent.SetWorldScale3D` _icon (`KismetMathLibrary.MakeVector` _returnvalue_2 _returnvalue_2 _returnvalue_2))
    (`BillboardComponent.SetSprite` (`self.Icon`) _newsprite))
  (if (> _timestoptimeleft 0.0)
    (set `self.TimeStopTimeLeft` (- _timestoptimeleft DeltaSeconds))
    (elif (<= _cooldown 0.0)
      (`SceneComponent.K2_SetWorldLocation` _platform (+ _returnvalue (* (`KismetMathLibrary.Normal` (- (`self.Target`) _returnvalue)) (* DeltaSeconds (`self.Speed`)))) false false)
      (if (< (`KismetMathLibrary.Vector_Distance` (`SceneComponent.K2_GetComponentLocation` _platform) (`self.Target`)) 5.0)
        (`SceneComponent.K2_SetWorldLocation` (`self.Destination`) (`self.Target`) false false)
        (set `self.Cooldown` (`self.CooldownLength`))
        (if (== (`self.Target`) (`self.PointB`))
          (set `self.Target` (`self.PointA`))
          (else
            (set `self.Target` (`self.PointB`)))))
      (else
        (set `self.Cooldown` (- _cooldown DeltaSeconds))))))

(fn `UserConstructionScript`)